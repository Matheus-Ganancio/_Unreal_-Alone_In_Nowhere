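; Interactable door actor that swings open or closed, or plays a rattle animation with a debug print when locked.
; Interact picks a Timeline from lock state and current yaw, choosing the opening direction from the player's relative look-at yaw.
; A DoOnce blocks repeat interaction until the animation finishes and resets it.
; TagSearch returns a locked or unlocked tag, noted as a DataTable key for icons.
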(event `/Game/Project/Blueprint/Interact/BPI_Interact_Interface.Interact`
  (bind (_relativerotation_roll _relativerotation_pitch _relativerotation_yaw) (`KismetMathLibrary.BreakRotator` (`SceneComponent.RelativeRotation` (`self.Door`))))
  (bind (_relativerotation_roll_2 _relativerotation_pitch_2 _relativerotation_yaw_2) (`KismetMathLibrary.BreakRotator` (`SceneComponent.RelativeRotation` (`self.Door`))))
  (bind (_returnvalue_roll _returnvalue_pitch _returnvalue_yaw) (`KismetMathLibrary.BreakRotator` (`KismetMathLibrary.FindRelativeLookAtRotation` (`self.GetTransform`) (`self.K2_GetActorLocation` (`GameplayStatics.GetPlayerCharacter` 0)))))
  ;[0.15 0.001393 0.000781 0.5] Confere se a porta esta trancada e caso sim realiza animacao
  (`/Engine/EditorBlueprintResources/StandardMacros.DoOnce` false :!label _label
    (:`Completed`
      (if (`self.Locked`)
        (`KismetSystemLibrary.PrintString` "Porta_Trancada")
        (bind (_direction _naoabre_porta) (`Timeline|Fechada_Porta` :!via `PlayFromStart`)
          (:`Update`
            (`SceneComponent.K2_SetRelativeRotation` (`self.Door`) (`KismetMathLibrary.MakeRotator` 0.0 0.0 _naoabre_porta) false false))
          (:`Finished`
            (`self.Reset_Door`)))
        (else
          ;[0.15 0.03325 0.1249 0.5] Animacao Fechamento Porta
          (if (or (>= _relativerotation_yaw 90.0) (<= _relativerotation_yaw -90.0))
            (if (>= _relativerotation_yaw_2 90.0)
              (set `self.Rotacao_Porta` (`self.Rotacao_Fora`))
              (bind (_direction_2 _fechar_rotacao) (`Timeline|Fechar_Porta` :!via `PlayFromStart` :!label _label_2)
                (:`Update`
                  (`SceneComponent.K2_SetRelativeRotation` (`self.Door`) (`KismetMathLibrary.MakeRotator` 0.0 0.0 (* _fechar_rotacao (`self.Rotacao_Porta`))) false false))
                (:`Finished`
                  (`self.Reset_Door`)))
              (else
                (set `self.Rotacao_Porta` (`self.Rotacao_Dentro`))
                (goto _label_2 :!via `PlayFromStart`)))
            (else
              ;[0.02755 0.02107 0.15 0.5] Usa a rotação da porta pra calcular a base do lado de abertura pela animação
              (if (<= _returnvalue_yaw 0.0)
                (set `self.Rotacao_Porta` (`self.Rotacao_Dentro`))
                (bind (_direction_3 `_rotação_abertura`) (`Timeline|Abrindo_Porta` :!via `PlayFromStart` :!label _label_3)
                  (:`Update`
                    (`SceneComponent.K2_SetRelativeRotation` (`self.Door`) (`KismetMathLibrary.MakeRotator` 0.0 0.0 (* `_rotação_abertura` (`self.Rotacao_Porta`))) false false))
                  (:`Finished`
                    (`self.Reset_Door`)))
                (else
                  (set `self.Rotacao_Porta` (`self.Rotacao_Fora`))
                  (goto _label_3 :!via `PlayFromStart`))))))))))

(event `Reset_Door`
  ;[0.15 0.001393 0.000781 0.5] Confere se a porta esta trancada e caso sim realiza animacao
  (goto _label :!via `Reset`))

(fn `TagSearch`
  (returns (tag :type Name))
  ; Verifica se a porta esta trancada, caso sim ele retorna o valor "Door_Locked" da datatable e caso não retorna "Door_Unlocked", no caso o valor de retorno seria icones
  (if (`self.Locked`)
    (return "Door_Locked")
    (else
      (return "Door_Unlocked"))))

(fn `UserConstructionScript`)