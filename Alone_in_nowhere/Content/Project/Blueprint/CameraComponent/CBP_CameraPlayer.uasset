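; Player camera component that applies a constant camera shake and sets depth-of-field post-process values.
; Every Tick starts the CBP_AnimCameraPlayer shake at reduced scale on the player camera manager and reassigns the post-process settings with fixed sensor width and focal distance.
; An unfinished DOF function traces forward on the Visibility channel but does nothing with the hit and is not called from the event graph.
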(event `self.ReceiveTick`
  (params (DeltaSeconds :type "Float (single-precision)"))
  (`PlayerCameraManager.StartCameraShake` :`self` (`GameplayStatics.GetPlayerCameraManager` 0) :`ShakeClass` "/Game/Project/Blueprint/CameraComponent/CBP_AnimCameraPlayer.CBP_AnimCameraPlayer_C" :`Scale` 0.3)
  (set `self.PostProcessSettings` (make `PostProcessSettings`)))

(fn `DOF`
  (bind _returnvalue (`self.K2_GetComponentLocation`))
  (bind (_outhit _returnvalue_2) (`KismetSystemLibrary.LineTraceSingle` _returnvalue (+ _returnvalue (* (`KismetMathLibrary.GetForwardVector` (`self.K2_GetComponentRotation`)) 10000.0)) "TraceTypeQuery1"))
  (if _returnvalue_2
    _))