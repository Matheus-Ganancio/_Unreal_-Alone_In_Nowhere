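; Enemy AI Blueprint that chases a sensed actor by sight and triggers game over on reaching it.
; AIPerception updates route stimuli by array index to vision or noise handlers; vision starts AIMoveTo, while noise has no response yet.
; A successful move fires a one-time GameOver that stops movement, shows WBP_Gameover, disables player input and switches to UI-only mode with cursor.
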(event `GameOver`
  (bind _returnvalue (`GameplayStatics.GetPlayerController` 0))
  ; Chama o gameover na tela
  (if (not (`self.bGameOverTriggered`))
    (set `self.bGameOverTriggered` true)
    (`Controller.StopMovement` (`self.GetController` self))
    (bind _returnvalue_2 (`|CreateWidget` "/Game/Project/HUD/WBP_Gameover.WBP_Gameover_C" _returnvalue))
    (bind _output_get (set `self.GameOverWidget` _returnvalue_2))
    (`UserWidget.AddToViewport` _output_get 0)
    (`WidgetBlueprintLibrary.SetInputMode_UIOnlyEx` (`GameplayStatics.GetPlayerController` 0) (`self.GameOverWidget`))
    (`self.DisableInput` (`GameplayStatics.GetPlayerCharacter` 0) null)
    (set `PlayerController.bShowMouseCursor` true _returnvalue)))

(event `Perception_Vision`
  (params (Actor :type "Actor Object Reference") (Stimulus :type "AIStimulus Structure"))
  ; Seguir player usando campo de visão
  (if (`.bSuccessfullySensed` (break `AIStimulus` Stimulus))
    (`|AIMoveTo` self (0.0 0.0 0.0) Actor 10.0 true
      (:`OnSuccess`
        (`self.GameOver`)))))

(event `self.AIPerception.OnPerceptionUpdated`
  (params (UpdatedActors :type "Array of Actor Object Reference (by ref)"))
  (for _array_element UpdatedActors
    (bind _info (`AIPerceptionComponent.GetActorsPerception` (`self.AIPerception`) _array_element))
    (bind (_target _lastsensedstimuli) (break `ActorPerceptionBlueprintInfo` _info))
    (for (_array_element_2 _array_index) _lastsensedstimuli
      (switch `int` _array_index
        (:`0`
          (`self.Perception_Vision` _target _array_element_2))
        (:`1`
          (`self.PerceptionNoise` _target _array_element_2))))))

(event `PerceptionNoise`
  (params (Actor :type "Actor Object Reference") (Stimulus :type "AIStimulus Structure"))
  (if (`.bSuccessfullySensed` (break `AIStimulus` Stimulus))
    _))

(fn `UserConstructionScript`)